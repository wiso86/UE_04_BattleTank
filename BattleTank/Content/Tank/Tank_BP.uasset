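; Tank pawn Blueprint that routes player input to movement, camera and firing.
; On BeginPlay it hands the barrel and turret to TankAiming and both tracks to TankMovement.
; Drive axes pass movement intent to TankMovement, and Fire calls TankAiming.
; Camera look splits yaw onto an azimuth gimbal and pitch onto the spring arm, each scaled by delta time and a sensitivity factor.
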(event EventBeginPlay
  (Class|TankAimingComponent|Initialise (Variables|Default|GetTankAiming) (Variables|Default|GetBarrel) (Variables|Default|GetTurret))
  (Class|TankMovementComponent|Initialise (Variables|Default|GetTankMovement) (Variables|Default|GetLeftTrack) (Variables|Default|GetRightTrack)))

(event Input|ActionEvents|InputActionFire
  (params (Key :type Key%20Structure :default "AnyKey"))
  ;[1 1 1] Camera input binding
  (:Pressed
    (Class|TankAimingComponent|Fire (Variables|Default|GetTankAiming))))

(event Input|AxisEvents|InputAxisAimAzimuth
  (params (AxisValue :type Float%20%28single-precision%29))
  ;[1 1 1] Camera input binding
  (Transformation|AddLocalRotation (Variables|Default|GetAzimuth%20Gimbal) (Math|Rotator|MakeRotator 0.0 0.0 (* AxisValue (Utilities|Time|GetWorldDeltaSeconds) (Variables|Input|GetAzimuth%20Scaling))) false false))

(event Input|AxisEvents|InputAxisAimElevation
  (params (AxisValue :type Float%20%28single-precision%29))
  ;[1 1 1] Camera input binding
  (Transformation|AddLocalRotation (Variables|Default|GetSpringArm) (Math|Rotator|MakeRotator 0.0 (* AxisValue (Utilities|Time|GetWorldDeltaSeconds) (Variables|Input|GetElevation%20Scaling)) 0.0) false false))

(event Input|AxisEvents|InputAxisTurnRight
  (params (AxisValue :type Float%20%28single-precision%29))
  ;[1 1 1] Movement binding
  (Class|TankMovementComponent|IntendMoveRight (Variables|Default|GetTankMovement) AxisValue))

(event Input|AxisEvents|InputAxisForward
  (params (AxisValue :type Float%20%28single-precision%29))
  ;[1 1 1] Movement binding
  (Class|TankMovementComponent|IntendMoveForward (Variables|Default|GetTankMovement) AxisValue))

(fn ConstructionScript)